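; RTS base game state that runs the in-game clock and calendar at an adjustable game speed.
; Each tick advances a Clockwork value, splits it into seconds, minutes and hours, rolls day ticks into months and years, and pushes both to the player controller's HUD.
; Speed changes scale the default time unit and pass it to CallUpdateGameSpeed.
; MakeBuilding, SetClockTime and SetDate are empty stubs.
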(event EventBeginPlay
  ;[1 1 1] Get reference to the player controller
  (bind _asrts_player_controller_bp (Utilities|Casting|CastToRTS_PlayerController_BP (Game|GetPlayerController 0)))
  (Variables|References|SetControllerRef _asrts_player_controller_bp)
  ;[1 1 1] Set custom date and time (default set at 1:1:1 & 1/1/1).
  (Variables|Default|SetClockwork (+ (Math|Conversions|ToFloat(Integer) (Variables|Default|GetSeconds)) (Math|Conversions|ToFloat(Integer) (Variables|Default|GetMinutes)) (Math|Conversions|ToFloat(Integer) (Variables|Default|GetHours))))
  (Variables|Default|SetGameDate (Utilities|Array|MakeArray (Variables|Default|GetDay) (Variables|Default|GetMonth) (Variables|Default|GetYear)))
  (Variables|References|SetRTSUIRef (Variables|/Game/_Gameplay/RTS_PlayerController_BP.RTS_PlayerController_BP_C|GetHUDRef (Variables|References|GetControllerRef)))
  (Variables|Default|SetTimeUnit (Variables|Default|GetDefaultGameSpeed)))

(event EventTick
  (params (DeltaSeconds :type Float%20%28single-precision%29))
  ;[1 1 1] Tick
  (Variables|Default|SetClockwork (.ClockworkOut (CallFunction|SetClockwork DeltaSeconds (Variables|Default|GetTimeUnit) (Variables|Default|GetClockwork))))
  (Variables|Default|SetDayTick (.DayTick (CallFunction|SetClockwork DeltaSeconds (Variables|Default|GetTimeUnit) (Variables|Default|GetClockwork))))
  (CallFunction|Clock)
  (CallFunction|Calendar))

(event EventUpdateGameStateSpeed
  (params (SpeedMultiplier :type Float%20%28single-precision%29))
  (bind _output_get (Variables|Default|SetTimeUnit (* SpeedMultiplier (Variables|Default|GetDefaultGameSpeed))))
  (Default|CallUpdateGameSpeed _output_get))

(fn ConstructionScript)

(fn Clock
  (bind _clockwork (Variables|Default|GetClockwork))
  (bind _returnvalue (* _clockwork 3.6e+03))
  (bind (_remainder _returnvalue_2) (Math|Float|Division(WholeandRemainder) _returnvalue 6e+01))
  (bind _returnvalue_3 (Math|Conversions|ToFloat(Integer) _returnvalue_2))
  (bind (_remainder_2 _returnvalue_4) (Math|Float|Division(WholeandRemainder) _returnvalue_3 6e+01))
  ;[1 1 1] 60 secs in a minute
  (Variables|Default|SetSeconds (Math|Float|Floor _remainder))
  ;[1 1 1] 60 mins in an hour
  (Variables|Default|SetMinutes (Math|Float|Floor _remainder_2))
  ;[1 1 1] 24 hours in a day
  (Variables|Default|SetHours (Math|Float|Floor (.Remainder (Math|Float|Division(WholeandRemainder) (Math|Conversions|ToFloat(Integer) _returnvalue_4) 24.0))))
  (bind _output_get (Variables|Default|SetGameTime (Utilities|Array|MakeArray (Variables|Default|GetSeconds) (Variables|Default|GetMinutes) (Variables|Default|GetHours))))
  (Class|RTSHUDI|SetClockTime(Message) (Variables|/Game/_Gameplay/RTS_PlayerController_BP.RTS_PlayerController_BP_C|GetHUDRef (Variables|References|GetControllerRef)) _output_get))

(fn Calendar
  (bind _output_get (Variables|Default|SetDay (+ (Variables|Default|GetDay) (Variables|Default|GetDayTick))))
  (if (> _output_get (Class|KismetMathLibrary|DaysinMonth (Variables|Default|GetYear) (Variables|Default|GetMonth)))
    (Variables|Default|SetDay 1)
    (Variables|Default|SetMonth (+ (Variables|Default|GetMonth) 1)))
  (if (> (Variables|Default|GetMonth) 12)
    (Variables|Default|SetMonth 1)
    (Variables|Default|SetYear (+ (Variables|Default|GetYear) 1)))
  (bind _output_get_2 (Variables|Default|SetGameDate (Utilities|Array|MakeArray (Variables|Default|GetDay) (Variables|Default|GetMonth) (Variables|Default|GetYear))))
  (Class|RTSHUDI|SetDate(Message) (Variables|/Game/_Gameplay/RTS_PlayerController_BP.RTS_PlayerController_BP_C|GetHUDRef (Variables|References|GetControllerRef)) _output_get_2))

(fn GetCurrentTimeUnit
  (return (Variables|Default|GetTimeUnit)))

(fn MakeBuilding
  (params (ConstructBuilding :type Bb%20Building%20Master%20BP%20Class%20Reference))
  (return))

(fn SetClockTime
  (params (Time :type Array%20of%20Integers))
  (return false))

(fn SetDate
  (params (Date :type Array%20of%20Integers))
  (return false))