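; Player controller for an RTS that drives the camera pawn, building placement, selection and pause menu.
; On BeginPlay it caches pawn and GameState references, spawns a construction manager and ghost building, and creates the HUD.
; In build mode, the ghost follows the cursor, rotates and queues construction when placeable; otherwise clicks send HUD requests.
; Camera speed scales with zoom, gates handle panning, edge scrolling is disconnected, and debug spawn keys remain.
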(event Custom|PauseMenu
  ;[1 1 1] Menus
  ;;[1 1 1] Pause Menu Call
  (Variables|Default|SetbShowMouseCursor true)
  (Game|SetGamePaused true)
  (bind _returnvalue (UserInterface|CreateWidget "/Game/_UI/Pause/BW_PauseMenu.BW_PauseMenu_C"))
  (UserInterface|Viewport|AddtoViewport _returnvalue 0))

(event Input|ActionEvents|InputActionSelect
  (params (Key :type Key%20Structure :default "None"))
  (bind _selectableobjects (Variables|Default|GetSelectableObjects))
  (bind _hitresult (Class|PlayerController|GetHitResultUnderCursorforObjects _selectableobjects true))
  (bind _hitactor (Collision|BreakHitResult _hitresult))
  ;[1 1 1] LMB Mouse Click
  (:Pressed
    (if (Variables|Default|GetisBuildModeActive)
      ;;[1 1 1] Building
      (if (|VerifyPlaceable)
        (bind _constructionstruct (Default|GetConstructionStruct (Variables|References|GetGhostBuildingRef)))
        (Default|QueueConstruction (Variables|References|GetConstructionManagerRef) _constructionstruct)
        (Default|KillGhostBuilding (Variables|References|GetGhostBuildingRef)))
      (else
        ;;[1 1 1] Display actor HUD tooltipstuff
        (if (!= _hitactor 0)
          (Default|CallHUDRequest _hitactor))))))

(event Input|ActionEvents|InputActionRotateBuildingLeft
  (params (Key :type Key%20Structure :default "None"))
  (bind _ghostbuildingref (Variables|References|GetGhostBuildingRef))
  (bind _returnvalue (Transformation|GetActorRotation _ghostbuildingref))
  (bind (_roll _pitch _yaw) (Math|Rotator|BreakRotator _returnvalue))
  ;[1 1 1] Rotate Buildings
  (:Pressed
    (if (and (Utilities|IsValid _ghostbuildingref) (Variables|Default|GetisBuildModeActive))
      (Transformation|SetActorRotation _ghostbuildingref (Math|Rotator|MakeRotator _roll _pitch (+ _yaw (Variables|Default|GetBuildingRotationRate)))))))

(event Input|ActionEvents|InputActionPanningReset
  (params (Key :type Key%20Structure :default "None"))
  (bind _camerapawnref (Variables|References|GetCameraPawnRef))
  (bind _returnvalue (Transformation|GetActorRotation _camerapawnref))
  (bind (_roll _pitch _yaw) (Math|Rotator|BreakRotator _returnvalue))
  ;[1 1 1] Movement
  ;;[1 1 1] Reset Panning
  (:Pressed
    (Transformation|SetActorRotation _camerapawnref (Math|Rotator|MakeRotator _roll 0.0 _yaw))))

(event Input|ActionEvents|InputActionZoomIn
  (params (Key :type Key%20Structure :default "None"))
  (bind _camerapawnref (Variables|References|GetCameraPawnRef))
  (bind _rtscameraarm (Variables|/Game/_Gameplay/RTS_CameraPawn_BP.RTS_CameraPawn_BP_C|GetRTSCameraArm _camerapawnref))
  ;[1 1 1] Movement
  ;;[1 1 1] Zoom in and out
  (:Pressed
    (Variables|/Script/Engine.SpringArmComponent|SetTargetArmLength _rtscameraarm (Math|Float|Clamp(Float) (- (Variables|/Script/Engine.SpringArmComponent|GetTargetArmLength _rtscameraarm) (Variables|Default|GetZoomSensitivity)) 5e+02 (Variables|Default|GetMaxArmLength)))))

(event Input|ActionEvents|InputActionZoomOut
  (params (Key :type Key%20Structure :default "None"))
  (bind _camerapawnref (Variables|References|GetCameraPawnRef))
  (bind _rtscameraarm (Variables|/Game/_Gameplay/RTS_CameraPawn_BP.RTS_CameraPawn_BP_C|GetRTSCameraArm _camerapawnref))
  ;[1 1 1] Movement
  ;;[1 1 1] Zoom in and out
  (:Pressed
    (Variables|/Script/Engine.SpringArmComponent|SetTargetArmLength _rtscameraarm (Math|Float|Clamp(Float) (+ (Variables|/Script/Engine.SpringArmComponent|GetTargetArmLength _rtscameraarm) (Variables|Default|GetZoomSensitivity)) 5e+02 (Variables|Default|GetMaxArmLength)))))

(event Input|ActionEvents|InputActionRotateBuildingRight
  (params (Key :type Key%20Structure :default "None"))
  (bind _ghostbuildingref (Variables|References|GetGhostBuildingRef))
  (bind _returnvalue (Transformation|GetActorRotation _ghostbuildingref))
  (bind (_roll _pitch _yaw) (Math|Rotator|BreakRotator _returnvalue))
  ;[1 1 1] Rotate Buildings
  (:Pressed
    (if (and (Utilities|IsValid _ghostbuildingref) (Variables|Default|GetisBuildModeActive))
      (Transformation|SetActorRotation _ghostbuildingref (Math|Rotator|MakeRotator _roll _pitch (- _yaw (Variables|Default|GetBuildingRotationRate)))))))

(event Input|ActionEvents|InputActionPanning
  (params (Key :type Key%20Structure :default "None"))
  (bind _camerapawnref (Variables|References|GetCameraPawnRef))
  (bind _returnvalue (Transformation|GetActorRotation _camerapawnref))
  (bind (_roll _pitch _yaw) (Math|Rotator|BreakRotator _returnvalue))
  ;[1 1 1] Movement
  ;;[1 1 1] Camera Panning X
  (:Pressed
    (Variables|Default|SetisDisableCamNav true)
    (Utilities|FlowControl|Gate true) ; enters at Open
  )
  (:Released
    (Variables|Default|SetisDisableCamNav false)
    (Utilities|FlowControl|Gate true) ; enters at Close
  ))

(event Input|ActionEvents|InputActionPanning
  (params (Key :type Key%20Structure :default "None"))
  (bind _camerapawnref (Variables|References|GetCameraPawnRef))
  (bind _returnvalue (Transformation|GetActorRotation _camerapawnref))
  (bind (_roll _pitch _yaw) (Math|Rotator|BreakRotator _returnvalue))
  ;[1 1 1] Movement
  ;;[1 1 1] Camera Panning Y
  (:Pressed
    (Variables|Default|SetisDisableCamNav true)
    (Utilities|FlowControl|Gate true) ; enters at Open
  )
  (:Released
    (Variables|Default|SetisDisableCamNav false)
    (Utilities|FlowControl|Gate true) ; enters at Close
  ))

(event Input|AxisEvents|InputAxisMoveForward
  (params (AxisValue :type Float%20%28single-precision%29))
  (bind _camerapawnref (Variables|References|GetCameraPawnRef))
  ;[1 1 1] Movement
  ;;[1 1 1] Movement X
  (if (not (Variables|Default|GetisDisableCamNav))
    (Transformation|SetActorTransform _camerapawnref (Utilities|MovementX (CallFunction|MovementSpeedCalculation) (Variables|Default|GetFastMoveMultiplier) AxisValue _camerapawnref))))

(event Input|AxisEvents|InputAxisMoveRight
  (params (AxisValue :type Float%20%28single-precision%29))
  (bind _movesensitivity (CallFunction|MovementSpeedCalculation))
  (bind _fastmovemultiplier (Variables|Default|GetFastMoveMultiplier))
  (bind _camerapawnref (Variables|References|GetCameraPawnRef))
  (bind _transform (Utilities|MovementY AxisValue _movesensitivity _fastmovemultiplier _camerapawnref))
  (bind (_location _rotation _scale) (Math|Transform|BreakTransform _transform))
  (bind (_x _y) (Math|Vector|BreakVector _location))
  ;[1 1 1] Movement
  ;;[1 1 1] Movement Y
  (if (not (Variables|Default|GetisDisableCamNav))
    (Transformation|SetActorTransform _camerapawnref (Math|Transform|MakeTransform (Math|Vector|MakeVector _x _y 1e+02) _rotation _scale))))

(event Input|MouseEvents|MouseX
  (params (AxisValue :type Float%20%28single-precision%29))
  (bind _camerapawnref (Variables|References|GetCameraPawnRef))
  (bind _returnvalue (Transformation|GetActorRotation _camerapawnref))
  (bind (_roll _pitch _yaw) (Math|Rotator|BreakRotator _returnvalue))
  ;[1 1 1] Movement
  ;;[1 1 1] Camera Panning X
  (Utilities|FlowControl|Gate true
    (:Exit
      (Transformation|SetActorRotation (Variables|References|GetCameraPawnRef) (Math|Rotator|MakeRotator _roll _pitch (+ _yaw (* (Variables|Default|GetPanSensitivity) AxisValue)))))))

(event Input|MouseEvents|MouseY
  (params (AxisValue :type Float%20%28single-precision%29))
  (bind _camerapawnref (Variables|References|GetCameraPawnRef))
  (bind _returnvalue (Transformation|GetActorRotation _camerapawnref))
  (bind (_roll _pitch _yaw) (Math|Rotator|BreakRotator _returnvalue))
  ;[1 1 1] Movement
  ;;[1 1 1] Camera Panning Y
  (Utilities|FlowControl|Gate true
    (:Exit
      (Transformation|SetActorRotation (Variables|References|GetCameraPawnRef) (Math|Rotator|MakeRotator _roll (Math|Float|Clamp(Float) (+ _pitch (* (Variables|Default|GetPanSensitivity) AxisValue)) -15.0 45.0) _yaw)))))

(event Input|MouseEvents|MouseX
  (params (AxisValue :type Float%20%28single-precision%29))
  ;[1 1 1] Movement
  ;;[1 0 0] Edge Scrolling - Currently Broken
)

(event Input|MouseEvents|MouseY
  (params (AxisValue :type Float%20%28single-precision%29))
  ;[1 1 1] Movement
  ;;[1 0 0] Edge Scrolling - Currently Broken
)

(event Input|KeyboardEvents|LeftShift
  (params (Key :type Key%20Structure :default "None"))
  ;[1 1 1] Movement
  ;;[1 1 1] Shift to move faster
  (:Pressed
    (Variables|Default|SetFastMoveMultiplier 2.0))
  (:Released
    (Variables|Default|SetFastMoveMultiplier 1.0)))

(event Input|KeyboardEvents|Escape
  (params (Key :type Key%20Structure :default "None"))
  ;[1 1 1] Menus
  ;;[1 1 1] Pause Menu Call
  (:Pressed
    (Variables|Default|SetbShowMouseCursor true)
    (Game|SetGamePaused true)
    (bind _returnvalue (UserInterface|CreateWidget "/Game/_UI/Pause/BW_PauseMenu.BW_PauseMenu_C"))
    (UserInterface|Viewport|AddtoViewport _returnvalue 0)))

(event Input|KeyboardEvents|U
  (params (Key :type Key%20Structure :default "None"))
  ;[1 0.5405 0] Debugging Camera - not complete
  (:Pressed
    (bind _returnvalue (Game|SpawnActorfromClass "/Script/Engine.DefaultPawn" (Transformation|GetActorTransform) "Undefined" 0 0))
    (Pawn|Possess (Game|GetPlayerController 0) _returnvalue)))

(event Input|KeyboardEvents|N
  (params (Key :type Key%20Structure :default "None"))
  (bind _self self)
  (bind _location (CallFunction|SetCursorWorldPos _self 1e+04))
  ;[1 0.9914 0] Temporary NPC Spawning
  (:Pressed
    (Game|SpawnActorfromClass "/Game/_NPCs/WorkerAI/NPC_BP.NPC_BP_C" (Math|Transform|MakeTransform (Math|Vector|MakeVector (.x _location) (.y _location) 93.0)) "Undefined" 0 (Variables|References|GetGameStateRef) 0)))

(event EventBeginPlay
  (bind _returnvalue (Math|Transform|MakeTransform "0, 0, 0"))
  (Utilities|FlowControl|Sequence
    (:then_0
      (Utilities|ReferenceCast))
    (:then_1
      (bind _returnvalue_2 (Game|SpawnActorfromClass "/Game/_Buildings/_Construction/bb_ConstructionManager_BP.bb_ConstructionManager_BP_C" _returnvalue "AlwaysSpawn" 0 0))
      (Variables|References|SetConstructionManagerRef _returnvalue_2))
    (:then_2
      (bind _returnvalue_3 (Game|SpawnActorfromClass "/Game/_Buildings/_Construction/bb_GhostBuilding_BP.bb_GhostBuilding_BP_C" _returnvalue "AlwaysSpawn" 0 self 0))
      (Variables|References|SetGhostBuildingRef _returnvalue_3))
    (:then_3
      (Variables|Default|SetbShowMouseCursor true)
      (Input|SetInputModeGameandUI self 0 "DoNotLock" false)
      (Utilities|CreateHUDs)
      (UserInterface|Viewport|AddtoViewport (Variables|References|GetHUDRef) 0))))

(event EventTick
  (params (DeltaSeconds :type Float%20%28single-precision%29))
  (if (Variables|Default|GetisBuildModeActive)
    (if (!= (Variables|References|GetGhostBuildingRef) 0)
      (Default|SetCursorPos (Variables|References|GetGhostBuildingRef) (CallFunction|SetCursorWorldPos self (CallFunction|SetBuildDistance))))))

(event Input|ActionEvents|InputActionDeselect
  (params (Key :type Key%20Structure))
  (:Pressed
    (if (Variables|Default|GetisBuildModeActive)
      (Default|KillGhostBuilding (Variables|References|GetGhostBuildingRef))
      (Variables|Default|SetisBuildModeActive false))))

(fn ConstructionScript)

(fn MovementSpeedCalculation
  (return (Math|Float|Clamp(Float) (/ (Variables|/Script/Engine.SpringArmComponent|GetTargetArmLength (Variables|/Game/_Gameplay/RTS_CameraPawn_BP.RTS_CameraPawn_BP_C|GetRTSCameraArm (Variables|References|GetCameraPawnRef))) 1e+02) 5.0 2e+01)))

(fn SetBuildDistance
  (return (+ (Variables|Default|GetBuildDistance) (Variables|/Script/Engine.SpringArmComponent|GetTargetArmLength (Variables|/Game/_Gameplay/RTS_CameraPawn_BP.RTS_CameraPawn_BP_C|GetRTSCameraArm (Variables|References|GetCameraPawnRef))))))

(fn SetClockTime
  (params (Time :type Array%20of%20Integers))
  (return false))

(fn SetDate
  (params (Date :type Array%20of%20Integers))
  (return false))