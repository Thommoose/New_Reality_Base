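; Worker AI NPC for an RTS that randomizes its sex, mesh, body colour and name profile in the construction script.
; Walk speed updates from the game state's speed-change dispatcher, and SetIsBusy writes to the AI blackboard.
; A player-controller HUD request opens the NPC's widget if it is visible, glides the camera pawn over by timeline, then a gated Tick keeps the camera following it.
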(event Custom|DisplayHUD
  (params (Actor :type Actor%20Object%20Reference))
  (bind _playercontrollerref (Variables|References|GetPlayerControllerRef))
  ;[1 1 1] Display HUD
  (if (and (== Actor self) (not (Variables|Rendering|GetbHidden)))
    (UserInterface|Viewport|AddtoViewport (Variables|References|GetNPC_HUD) 0)
    (Input|SetInputModeUIOnly _playercontrollerref 0 "LockInFullscreen")
    (Widget|SetIsEnabled (Variables|/Game/_Gameplay/RTS_PlayerController_BP.RTS_PlayerController_BP_C|GetHUDRef _playercontrollerref) false)
    (bind _newlocation (|CollapseGraph_0 (Variables|/Game/_Gameplay/RTS_PlayerController_BP.RTS_PlayerController_BP_C|GetCameraPawnRef _playercontrollerref))
      (:Update
        (Transformation|SetActorLocation (Variables|/Game/_Gameplay/RTS_PlayerController_BP.RTS_PlayerController_BP_C|GetCameraPawnRef (Variables|References|GetPlayerControllerRef)) _newlocation false false))
      (:Finished
        (Variables|/Game/_Gameplay/RTS_PlayerController_BP.RTS_PlayerController_BP_C|SetisDisableCamNav (Variables|References|GetPlayerControllerRef) true)
        (CallFunction|OpenFollowGate)))))

(event Custom|OpenFollowGate
  (bind _returnvalue (Transformation|GetActorLocation))
  (bind _playercontrollerref (Variables|References|GetPlayerControllerRef))
  (bind _camerapawnref (Variables|/Game/_Gameplay/RTS_PlayerController_BP.RTS_PlayerController_BP_C|GetCameraPawnRef _playercontrollerref))
  ;[1 1 1] Follow the NPC when UI is open
  (Utilities|FlowControl|Gate true) ; enters at Open
)

(event Custom|CloseFollowGate
  (bind _returnvalue (Transformation|GetActorLocation))
  (bind _playercontrollerref (Variables|References|GetPlayerControllerRef))
  (bind _camerapawnref (Variables|/Game/_Gameplay/RTS_PlayerController_BP.RTS_PlayerController_BP_C|GetCameraPawnRef _playercontrollerref))
  ;[1 1 1] Follow the NPC when UI is open
  (Utilities|FlowControl|Gate true) ; enters at Close
)

(event Custom|UpdateWalkingSpeed
  (params (TimeUnit :type Float%20%28single-precision%29))
  ;[1 1 1] Alter Walking speed Event. Time unit is not used but needs to be called as its a message dispatch.
  (Variables|/Script/Engine.CharacterMovementComponent|SetMaxWalkSpeed (Variables|Character|GetCharacterMovement) (/ (Variables|Default|GetBaseWalkSpeed) (Variables|/Game/_Gameplay/RTS_GamestateBase_BP.RTS_GamestateBase_BP_C|GetSpeed%20Multiplier (Variables|References|GetGameStateRef)))))

(event EventBeginPlay
  ;[1 1 1] Begin Play
  (bind _asnpc_ai_controller_bp (Utilities|Casting|CastToNPC_AI_Controller_BP (AI|GetAIController self)))
  (Variables|References|SetAIControlerRef _asnpc_ai_controller_bp)
  (bind _asrts_player_controller_bp (Utilities|Casting|CastToRTS_PlayerController_BP (Game|GetPlayerController 0)))
  (bind _output_get (Variables|References|SetPlayerControllerRef _asrts_player_controller_bp))
  (EventDispatchers|BindEventtoHUDRequest _output_get (EventDispatchers|CreateEvent :!event Custom|DisplayHUD))
  (bind _returnvalue (UserInterface|CreateWidget "/Game/_UI/HUDs/RTS_NPC_HUD.RTS_NPC_HUD_C" 0 self))
  (Variables|References|SetNPC_HUD _returnvalue)
  (EventDispatchers|BindEventtoUpdateGameSpeed (Variables|References|GetGameStateRef) (EventDispatchers|CreateEvent :!event Custom|UpdateWalkingSpeed)))

(event EventTick
  (params (DeltaSeconds :type Float%20%28single-precision%29))
  (bind _returnvalue (Transformation|GetActorLocation))
  (bind _playercontrollerref (Variables|References|GetPlayerControllerRef))
  (bind _camerapawnref (Variables|/Game/_Gameplay/RTS_PlayerController_BP.RTS_PlayerController_BP_C|GetCameraPawnRef _playercontrollerref))
  ;[1 1 1] Follow the NPC when UI is open
  (Utilities|FlowControl|Gate true
    (:Exit
      (Transformation|SetActorLocation _camerapawnref (Math|Vector|MakeVector (.x _returnvalue) (.y _returnvalue) (.z (Transformation|GetActorLocation _camerapawnref))) false false))))

(fn ConstructionScript
  (CallFunction|RandomNPCFeatures))

(fn RandomNPCFeatures
  (bind _mesh (Variables|Character|GetMesh))
  (bind _mesh_2 (Variables|Character|GetMesh))
  (bind _mesh_3 (Variables|Character|GetMesh))
  (bind _output_get (LocalVariables|SetRandomSex (Utilities|Enum|ByteToEnumNPC_Sex_ENUM (Math|Conversions|ToByte(Integer) (Math|Random|RandomIntegerinRange 0 2)))))
  (if (Utilities|Enum|Equal(Enum) _output_get "NewEnumerator0")
    (Class|SkinnedMeshComponent|SetSkeletalMesh _mesh_2 "/Game/Mannequin/Character/Mesh/SK_Mannequin.SK_Mannequin" true)
    (bind _returnvalue (Rendering|Material|CreateDynamicMaterialInstance _mesh_2 0 "/Game/Mannequin/Character/Materials/M_Male_Body_Inst.M_Male_Body_Inst" "None" :!class /Script/Engine.PrimitiveComponent))
    (bind _output_get_2 (LocalVariables|SetMaleMaterialInstance _returnvalue))
    (Rendering|Material|SetVectorParameterValue _output_get_2 (LocalVariables|GetBodyColor) (LocalVariables|GetMaleColour) :!class /Script/Engine.MaterialInstanceDynamic)
    (bind _name (CallFunction|GetRandomFirstName "NewEnumerator0"))
    (bind _name_2 (CallFunction|GetRandomSurname))
    (bind _output_get_3 (Variables|Default|SetMyProfile (Utilities|Struct|MakeNPC_Profile_Struct _name _name_2 "NewEnumerator0")))
    ;[1 0.6161 0] Debugging Issues
    (Development|PrintString (Utilities|String|Append (Utilities|String|Append (.fName (Utilities|Struct|BreakNPC_Profile_Struct _output_get_3)) "   " (.sName (Utilities|Struct|BreakNPC_Profile_Struct _output_get_3))) "     " (Utilities|String|EnumtoString (.Sex (Utilities|Struct|BreakNPC_Profile_Struct _output_get_3)))))
    (elif (Utilities|Enum|Equal(Enum) _output_get "NewEnumerator1")
      (Class|SkinnedMeshComponent|SetSkeletalMesh _mesh_3 "/Game/Mannequin/Character/Mesh/SK_Mannequin_Female.SK_Mannequin_Female" true)
      (bind _returnvalue_2 (Rendering|Material|CreateDynamicMaterialInstance _mesh_3 0 "/Game/Mannequin/Character/Materials/M_Female_Body_Inst.M_Female_Body_Inst" "None" :!class /Script/Engine.PrimitiveComponent))
      (bind _output_get_4 (LocalVariables|SetFemaleMaterialInstance _returnvalue_2))
      (Rendering|Material|SetVectorParameterValue _output_get_4 (LocalVariables|GetBodyColor) (LocalVariables|GetFemaleColour) :!class /Script/Engine.MaterialInstanceDynamic)
      (bind _name_3 (CallFunction|GetRandomFirstName "NewEnumerator1"))
      (bind _name_4 (CallFunction|GetRandomSurname))
      (bind _output_get_5 (Variables|Default|SetMyProfile (Utilities|Struct|MakeNPC_Profile_Struct _name_3 _name_4 "NewEnumerator1")))
      (Development|PrintString (Utilities|String|Append (Utilities|String|Append (.fName (Utilities|Struct|BreakNPC_Profile_Struct _output_get_5)) "   " (.sName (Utilities|Struct|BreakNPC_Profile_Struct _output_get_5))) "     " (Utilities|String|EnumtoString (.Sex (Utilities|Struct|BreakNPC_Profile_Struct _output_get_5)))) true true "(R=1.000000,G=0.101204,B=0.966796,A=1.000000)")
      (else
        (Class|SkinnedMeshComponent|SetSkeletalMesh _mesh "/Game/Mannequin/Character/Mesh/SK_Mannequin.SK_Mannequin" true)
        (Transformation|SetWorldScale3D _mesh "0.750000,0.750000,0.750000")
        (bind _returnvalue_3 (Rendering|Material|CreateDynamicMaterialInstance _mesh 0 "/Game/Mannequin/Character/Materials/M_Male_Body_Inst.M_Male_Body_Inst" "None" :!class /Script/Engine.PrimitiveComponent))
        (bind _output_get_6 (LocalVariables|SetMaleMaterialInstance _returnvalue_3))
        (Rendering|Material|SetVectorParameterValue _output_get_6 (LocalVariables|GetBodyColor) (LocalVariables|GetGenderlessColour) :!class /Script/Engine.MaterialInstanceDynamic)
        (bind _name_5 (CallFunction|GetRandomFirstName "NewEnumerator2"))
        (bind _name_6 (CallFunction|GetRandomSurname))
        (bind _output_get_7 (Variables|Default|SetMyProfile (Utilities|Struct|MakeNPC_Profile_Struct _name_5 _name_6 "NewEnumerator2")))
        (Development|PrintString (Utilities|String|Append (Utilities|String|Append (.fName (Utilities|Struct|BreakNPC_Profile_Struct _output_get_7)) "   " (.sName (Utilities|Struct|BreakNPC_Profile_Struct _output_get_7))) "     " (Utilities|String|EnumtoString (.Sex (Utilities|Struct|BreakNPC_Profile_Struct _output_get_7)))) true true "(R=0.004949,G=1.000000,B=0.019227,A=1.000000)")))))

(fn GetRandomFirstName
  (params (Sex :type NPC_Sex_ENUM%20Enum :default "NewEnumerator0"))
  (bind _returnvalue (|GetNumEnumEntries))
  (bind _returnvalue_2 (|GetNumEnumEntries))
  (bind _returnvalue_3 (- _returnvalue_2 1))
  (bind _returnvalue_4 (- _returnvalue 1))
  (bind _returnvalue_5 (Math|Random|RandomIntegerinRange 0 _returnvalue_3))
  (bind _returnvalue_6 (Math|Random|RandomIntegerinRange 0 _returnvalue_4))
  (bind _returnvalue_7 (Math|Conversions|ToByte(Integer) _returnvalue_5))
  (bind _returnvalue_8 (Math|Conversions|ToByte(Integer) _returnvalue_6))
  (bind _returnvalue_9 (Utilities|Enum|ByteToEnumNPC_fName_Male_ENUM _returnvalue_8))
  (bind _returnvalue_10 (Utilities|Enum|ByteToEnumNPC_fName_Female_ENUM _returnvalue_7))
  (bind _returnvalue_11 (Utilities|String|EnumtoString _returnvalue_9))
  (bind _returnvalue_12 (Utilities|String|EnumtoString _returnvalue_10))
  (if (Utilities|Enum|Equal(Enum) Sex "NewEnumerator0")
    (return _returnvalue_11)
    (elif (Utilities|Enum|Equal(Enum) Sex "NewEnumerator1")
      (return _returnvalue_12)
      (elif (== (Math|Random|RandomIntegerinRange 0 1) 0)
        (return _returnvalue_11)
        (else
          (return _returnvalue_12))))))

(fn SetIsBusy
  (params (isBusy :type Boolean))
  (AI|Components|Blackboard|SetValueasBool (AI|GetBlackboard (Variables|References|GetAIControlerRef)) (Variables|Default|GetisBusy) isBusy)
  (return))

(fn GetRandomSurname
  (return (Utilities|String|EnumtoString (Utilities|Enum|ByteToEnumNPC_sName_ENUM (Math|Conversions|ToByte(Integer) (Math|Random|RandomIntegerinRange 0 (- (|GetNumEnumEntries) 1)))))))