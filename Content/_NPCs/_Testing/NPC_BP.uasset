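; Randomised RTS NPC that gets a sex, matching mannequin mesh, tinted body material and name profile in its construction script.
; Names are drawn from enums used as name pools; the third, genderless option uses a scaled-down male mesh and either name pool.
; BeginPlay binds to the player controller's HUD request, showing its own widget when selected by that event.
; Helpers set the AI blackboard's busy flag and create a scene-capture portrait render target and material.
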(event Custom|DisplayHUD
  (params (Actor :type Actor%20Object%20Reference))
  (if (== Actor self)
    (UserInterface|Viewport|AddtoViewport (Variables|Default|GetNPC_HUD) 0)))

(event EventBeginPlay
  (bind _asnpc_ai_controller_bp (Utilities|Casting|CastToNPC_AI_Controller_BP (AI|GetAIController self)))
  (Variables|References|SetAIControlerRef _asnpc_ai_controller_bp)
  (bind _asrts_player_controller_bp (Utilities|Casting|CastToRTS_PlayerController_BP (Game|GetPlayerController 0)))
  (bind _output_get (Variables|Default|SetPlayerControllerRef _asrts_player_controller_bp))
  (EventDispatchers|BindEventtoHUDRequest _output_get (EventDispatchers|CreateEvent :!event Custom|DisplayHUD))
  (bind _returnvalue (UserInterface|CreateWidget "/Game/_UI/HUDs/RTS_NPC_HUD.RTS_NPC_HUD_C" 0 self 0 0))
  (Variables|Default|SetNPC_HUD _returnvalue))

(fn ConstructionScript
  (CallFunction|RandomNPCFeatures))

(fn RandomNPCFeatures
  (bind _mesh (Variables|Character|GetMesh))
  (bind _mesh_2 (Variables|Character|GetMesh))
  (bind _mesh_3 (Variables|Character|GetMesh))
  (bind _output_get (LocalVariables|SetRandomSex (Utilities|Enum|ByteToEnumNPC_Sex_ENUM (Math|Conversions|ToByte(Integer) (Math|Random|RandomIntegerinRange 0 2)))))
  (if (Utilities|Enum|Equal(Enum) _output_get "NewEnumerator0")
    (Class|SkinnedMeshComponent|SetSkeletalMesh _mesh_2 "/Game/Mannequin/Character/Mesh/SK_Mannequin.SK_Mannequin" true)
    (bind _returnvalue (Rendering|Material|CreateDynamicMaterialInstance _mesh_2 0 "/Game/Mannequin/Character/Materials/M_Male_Body_Inst.M_Male_Body_Inst" "None" :!class /Script/Engine.PrimitiveComponent))
    (bind _output_get_2 (LocalVariables|SetMaleMaterialInstance _returnvalue))
    (Rendering|Material|SetVectorParameterValue _output_get_2 (LocalVariables|GetBodyColor) (LocalVariables|GetMaleColour) :!class /Script/Engine.MaterialInstanceDynamic)
    (bind _name (CallFunction|GetRandomFirstName "NewEnumerator0"))
    (bind _name_2 (CallFunction|GetRandomSurname))
    (Variables|Default|SetMyProfile (Utilities|Struct|MakeNPC_Profile_Struct _name _name_2 "NewEnumerator0"))
    (elif (Utilities|Enum|Equal(Enum) _output_get "NewEnumerator1")
      (Class|SkinnedMeshComponent|SetSkeletalMesh _mesh_3 "/Game/Mannequin/Character/Mesh/SK_Mannequin_Female.SK_Mannequin_Female" true)
      (bind _returnvalue_2 (Rendering|Material|CreateDynamicMaterialInstance _mesh_3 0 "/Game/Mannequin/Character/Materials/M_Female_Body_Inst.M_Female_Body_Inst" "None" :!class /Script/Engine.PrimitiveComponent))
      (bind _output_get_3 (LocalVariables|SetFemaleMaterialInstance _returnvalue_2))
      (Rendering|Material|SetVectorParameterValue _output_get_3 (LocalVariables|GetBodyColor) (LocalVariables|GetFemaleColour) :!class /Script/Engine.MaterialInstanceDynamic)
      (bind _name_3 (CallFunction|GetRandomFirstName "NewEnumerator1"))
      (bind _name_4 (CallFunction|GetRandomSurname))
      (Variables|Default|SetMyProfile (Utilities|Struct|MakeNPC_Profile_Struct _name_3 _name_4 "NewEnumerator1"))
      (else
        (Class|SkinnedMeshComponent|SetSkeletalMesh _mesh "/Game/Mannequin/Character/Mesh/SK_Mannequin.SK_Mannequin" true)
        (Transformation|SetWorldScale3D _mesh "0.750000,0.750000,0.750000")
        (bind _returnvalue_3 (Rendering|Material|CreateDynamicMaterialInstance _mesh 0 "/Game/Mannequin/Character/Materials/M_Male_Body_Inst.M_Male_Body_Inst" "None" :!class /Script/Engine.PrimitiveComponent))
        (bind _output_get_4 (LocalVariables|SetMaleMaterialInstance _returnvalue_3))
        (Rendering|Material|SetVectorParameterValue _output_get_4 (LocalVariables|GetBodyColor) (LocalVariables|GetGenderlessColour) :!class /Script/Engine.MaterialInstanceDynamic)
        (bind _name_5 (CallFunction|GetRandomFirstName "NewEnumerator2"))
        (bind _name_6 (CallFunction|GetRandomSurname))
        (Variables|Default|SetMyProfile (Utilities|Struct|MakeNPC_Profile_Struct _name_5 _name_6 "NewEnumerator2"))))))

(fn GetRandomFirstName
  (params (Sex :type NPC_Sex_ENUM%20Enum :default "NewEnumerator0"))
  (bind _returnvalue (|GetNumEnumEntries))
  (bind _returnvalue_2 (|GetNumEnumEntries))
  (bind _returnvalue_3 (- _returnvalue_2 1))
  (bind _returnvalue_4 (- _returnvalue 1))
  (bind _returnvalue_5 (Math|Random|RandomIntegerinRange 0 _returnvalue_3))
  (bind _returnvalue_6 (Math|Random|RandomIntegerinRange 0 _returnvalue_4))
  (bind _returnvalue_7 (Math|Conversions|ToByte(Integer) _returnvalue_5))
  (bind _returnvalue_8 (Math|Conversions|ToByte(Integer) _returnvalue_6))
  (bind _returnvalue_9 (Utilities|Enum|ByteToEnumNPC_fName_Male_ENUM _returnvalue_8))
  (bind _returnvalue_10 (Utilities|Enum|ByteToEnumNPC_fName_Female_ENUM _returnvalue_7))
  (bind _returnvalue_11 (Utilities|Enum|LiteralenumNPC_fName_Male_ENUM _returnvalue_9))
  (bind _returnvalue_12 (Utilities|Enum|LiteralenumNPC_fName_Female_ENUM _returnvalue_10))
  (bind _returnvalue_13 (Utilities|String|EnumtoString _returnvalue_11))
  (bind _returnvalue_14 (Utilities|String|EnumtoString _returnvalue_12))
  (if (Utilities|Enum|Equal(Enum) Sex "NewEnumerator0")
    (return _returnvalue_13)
    (elif (Utilities|Enum|Equal(Enum) Sex "NewEnumerator1")
      (return _returnvalue_14)
      (elif (== (Math|Random|RandomIntegerinRange 0 1) 0)
        (return _returnvalue_13)
        (else
          (return _returnvalue_14))))))

(fn SetIsBusy
  (params (isBusy :type Boolean))
  (AI|Components|Blackboard|SetValueasBool (AI|GetBlackboard (Variables|References|GetAIControlerRef)) (Variables|Default|GetisBusy) isBusy)
  (return))

(fn GetRandomSurname
  (return (Utilities|String|EnumtoString (Utilities|Enum|LiteralenumNPC_sName_ENUM (Utilities|Enum|ByteToEnumNPC_sName_ENUM (Math|Conversions|ToByte(Integer) (Math|Random|RandomIntegerinRange 0 (- (|GetNumEnumEntries) 1))))))))

(fn GetPortrait
  (bind _returnvalue (Rendering|CreateRenderTarget2D 256 256 "RTF_RGBA16f"))
  (bind _output_get (LocalVariables|SetPortraitRenderTarget _returnvalue))
  (bind _output_get_2 (Variables|/Script/Engine.SceneCaptureComponent2D|SetTextureTarget (Variables|Default|GetNPCPortraitCapture) _output_get))
  (bind _returnvalue_2 (Rendering|Material|CreateDynamicMaterialInstance "/Game/_NPCs/_Testing/AI/NPC_Portrait_M_Inst.NPC_Portrait_M_Inst" "None" "None" :!class /Script/Engine.KismetMaterialLibrary))
  (bind _output_get_3 (Variables|Default|SetPortraitMaterial _returnvalue_2))
  (return _output_get_2 _output_get_3))